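; Player cat character Blueprint that relays notifications to the HUD and handles a return to the title screen.
; BeginPlay caches the main HUD from the cat controller.
; OnNotifyPlayer swishes the message into that HUD's stat bar widget, then swishes it out after the widget's notification delay.
; Releasing the Title input deletes the main save slot before opening the title level, so saved progress is wiped.
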(event EventBeginPlay
  (bind _asbp_cat_controller (Utilities|Casting|CastToBP_CatController (Game|GetPlayerController 0)))
  (Variables|Default|SetCat%20Main%20HUD (Variables|/Game/Blueprints/Character/Controller/BP_CatController.BP_CatController_C|GetCatMainHUD _asbp_cat_controller)))

(event Collision|EventActorBeginOverlap
  (params (OtherActor :type Actor%20Object%20Reference)))

(event EventTick
  (params (DeltaSeconds :type Float%20%28single-precision%29)))

(event EventOnNotifyPlayer
  (params (Notification :type String))
  (bind _asbp_stat_bar_widget (Utilities|Casting|CastToBP_StatBarWidget (Variables|/Script/CatsMeow.CatMainHUD|GetStatBarWidgetInstance (Variables|Default|GetCat%20Main%20HUD))))
  (Default|SwishinNotification _asbp_stat_bar_widget (Utilities|Text|ToText(String) Notification))
  (Utilities|FlowControl|Delay (Variables|/Game/Blueprints/UI_Widgets/BP_StatBarWidget.BP_StatBarWidget_C|GetNotificationDelay _asbp_stat_bar_widget))
  (Default|SwishOutNotification _asbp_stat_bar_widget))

(event Input|ActionEvents|InputActionTitle
  (params (Key :type Key%20Structure :default "None"))
  (:Released
    (SaveGame|DeleteGameinSlot "MainSlot")
    (Game|OpenLevel(byName) "TitleScreen")))

(fn ConstructionScript)